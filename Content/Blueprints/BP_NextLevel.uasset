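; BP_NextLevel is a level exit that appears once no BP_BlackBlueEnemy actors remain and sends the player to the next level.
; It starts with a hidden Cube and a collisionless Box, polls for enemies every Tick, then enables both and plays a scale Timeline on the Cube.
; An FPSCharacter overlapping the enabled Box opens the next numbered level from MyGameInstance's CurrentLevel, or Map_EndGame after the fifth.
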(event OnComponentBeginOverlap(Box)
  (params (OverlappedComponent :type Primitive%20Component%20Object%20Reference) (OtherActor :type Actor%20Object%20Reference) (OtherComp :type Primitive%20Component%20Object%20Reference) (OtherBodyIndex :type Integer) (bFromSweep :type Boolean) (SweepResult :type Hit%20Result%20Structure%20%28by%20ref%29))
  (bind _returnvalue (Game|GetGameInstance))
  (bind _asmy_game_instance (Utilities|Casting|CastToMyGameInstance _returnvalue))
  (bind _currentlevel (Variables|/Game/Blueprints/MyGameInstance.MyGameInstance_C|GetCurrentLevel _asmy_game_instance))
  ;[1 1 1] Open Level
  (if (Variables|Default|GetEnable)
    (Utilities|Casting|CastToFPSCharacter OtherActor)
    (if (== _currentlevel 5)
      (Game|OpenLevel(byName) "Map_EndGame")
      (else
        (Game|OpenLevel(byName) (Utilities|String|StringToName (Utilities|String|Append "Level" (Utilities|String|ToString(Integer) (+ _currentlevel 1)))))))))

(event EventBeginPlay
  ;[1 1 1] Hide actor
  (Rendering|SetVisibility (Variables|Default|GetCube) false false)
  (Collision|SetCollisionEnabled (Variables|Default|GetBox) "NoCollision"))

(event EventTick
  (params (DeltaSeconds :type Float%20%28single-precision%29))
  ;[1 1 1] Check is ready
  (bind _outactors (Actor|GetAllActorsOfClass "/Game/Blueprints/BP_BlackBlueEnemy.BP_BlackBlueEnemy_C"))
  (if (== (Utilities|Array|Length _outactors) 0)
    (Rendering|SetVisibility (Variables|Default|GetCube) true false)
    (Collision|SetCollisionEnabled (Variables|Default|GetBox) "QueryAndPhysics")
    (Variables|Default|SetEnable true)
    (bind _scale (Timeline|Timeline_0 Play)
      (:Update
        (Transformation|SetRelativeScale3D (Variables|Default|GetCube) (* "1.000000,1.000000,1.000000" _scale))))))

(fn ConstructionScript)