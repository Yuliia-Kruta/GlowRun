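; BP_Bullet is a projectile actor that flies at a configurable speed and destroys itself after its lifetime expires.
; On BeginPlay it applies the speed to its projectile movement and a configurable material to its mesh.
; When its box overlaps anything other than the player character, gun, other bullets or a BlackBlue enemy collision actor, it spawns a hit particle in that material and destroys itself after a tiny delay.
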(event OnComponentBeginOverlap(Box)
  (params (OverlappedComponent :type Primitive%20Component%20Object%20Reference) (OtherActor :type Actor%20Object%20Reference) (OtherComp :type Primitive%20Component%20Object%20Reference) (OtherBodyIndex :type Integer) (bFromSweep :type Boolean) (SweepResult :type Hit%20Result%20Structure%20%28by%20ref%29))
  (bind _returnvalue (Utilities|GetClass OtherActor))
  (bind _defaultsceneroot (Variables|Default|GetDefaultSceneRoot))
  (bind _returnvalue_2 (Transformation|GetWorldTransform _defaultsceneroot))
  ;[1 1 1] Hit
  (if (Math|Boolean|ANDBoolean (!= _returnvalue "/Game/Blueprints/FPSCharacter.FPSCharacter_C") (!= _returnvalue "/Game/Blueprints/BP_Gun.BP_Gun_C") (!= _returnvalue "BP_Bullet_C") (!= _returnvalue "/Game/Blueprints/BP_BlackBlueEnemyCollision.BP_BlackBlueEnemyCollision_C"))
    (bind _returnvalue_3 (Effects|SpawnEmitteratLocation "/Game/Widgets/HitParticleSystem.HitParticleSystem" (.location _returnvalue_2) (.rotation _returnvalue_2) (.scale _returnvalue_2)))
    (Rendering|Material|SetMaterial _returnvalue_3 0 (Variables|Default|GetMat))
    (Utilities|FlowControl|Delay 0.01)
    (Actor|DestroyActor)))

(event EventBeginPlay
  (bind _projectilemovement (Variables|Default|GetProjectileMovement))
  (bind _speed (Variables|Default|GetSpeed))
  ;[1 1 1] BeginPlay
  (Variables|/Script/Engine.ProjectileMovementComponent|SetInitialSpeed _projectilemovement _speed)
  (Variables|/Script/Engine.ProjectileMovementComponent|SetMaxSpeed _projectilemovement _speed)
  (Rendering|Material|SetMaterial (Variables|Default|GetStaticMesh) 0 (Variables|Default|GetMat))
  (Utilities|FlowControl|Delay (Variables|Default|GetLifetime))
  (Actor|DestroyActor))

(fn ConstructionScript)