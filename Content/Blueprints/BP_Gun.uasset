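; BP_Gun is a gun actor that spawns a BP_Bullet when its Fire event is called.
; Fire line-traces forward from the root, then picks the hit location or a fallback point straight ahead as the target.
; The bullet spawns at the Scene component, rotated by the root-to-target look-at, with a blue material and character-ignore enabled.
; A disconnected green-bullet spawn without the trace never runs.
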(event Custom|Fire
  (bind _defaultsceneroot (Variables|Default|GetDefaultSceneRoot))
  (bind _scene (Variables|Default|GetScene))
  (bind _returnvalue (Math|Vector|GetForwardVector _defaultsceneroot))
  (bind _returnvalue_2 (Transformation|GetWorldLocation _defaultsceneroot))
  (bind _returnvalue_3 (Transformation|GetWorldTransform _scene))
  ;[1 1 1] Find shoot trajectory
  (bind (_outhit _returnvalue_4) (Collision|LineTraceForObjects _returnvalue_2 (+ _returnvalue_2 (* _returnvalue 1e+04)) (Utilities|Array|MakeArray "ObjectTypeQuery1" "ObjectTypeQuery2" "ObjectTypeQuery4") false 0 "None"))
  (Game|SpawnActorfromClass "/Game/Blueprints/BP_Bullet.BP_Bullet_C" (Math|Transform|MakeTransform (.location _returnvalue_3) (Math|Rotator|FindLookatRotation _returnvalue_2 (Math|Vector|SelectVector (.location _outhit) (+ _returnvalue_2 (* _returnvalue 1e+03)) _returnvalue_4)) (.scale _returnvalue_3)) "Undefined" 0 "/Game/Blueprints/Material/M_Blue2_Inst.M_Blue2_Inst" 1e+04 true 4.0 2e+01 0))

(fn ConstructionScript)