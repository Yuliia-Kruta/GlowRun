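; BP_Enemy is a shooting enemy whose Sphere turns toward the player character every tick.
; Animate reveals it and runs a one-time timeline that moves and scales it, then starts a delay loop spawning BP_Bullet from Scene1.
; Shoot and StopShoot play scale timelines and toggle the LookOnCharacter flag gating that loop.
; BP_Bullet overlaps on Sphere1 reduce HP, destroying the enemy at zero.
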(event OnComponentBeginOverlap(Sphere1)
  (params (OverlappedComponent :type Primitive%20Component%20Object%20Reference) (OtherActor :type Actor%20Object%20Reference) (OtherComp :type Primitive%20Component%20Object%20Reference) (OtherBodyIndex :type Integer) (bFromSweep :type Boolean) (SweepResult :type Hit%20Result%20Structure%20%28by%20ref%29))
  ;[1 1 1] Apply damage
  (Utilities|Casting|CastToBP_Bullet OtherActor)
  (bind _output_get (Variables|Default|SetHP (- (Variables|Default|GetHP) 1e+01)))
  (if (<= _output_get 0.0)
    (Actor|DestroyActor)))

(event Custom|Shoot
  (bind _scene (Variables|Default|GetScene))
  ;[1 1 1] ShootAnimate
  (bind _scale (Timeline|Timeline_1 PlayFromStart)
    (:Update
      (Transformation|SetWorldTransform _scene (Math|Transform|MakeTransform (Transformation|GetWorldLocation _scene) (Transformation|GetWorldRotation _scene) (* "1.000000,1.000000,1.000000" _scale)) false false))
    (:Finished
      ;[1 1 1] Shoot
      (bind _output_get (Variables|Default|SetLookOnCharacter true))
      (if _output_get :!label _label
        (Utilities|FlowControl|Delay 0.5)
        (Game|SpawnActorfromClass "/Game/Blueprints/BP_Bullet.BP_Bullet_C" (Transformation|GetWorldTransform (Variables|Default|GetScene1)) "Undefined" 0 "/Game/Blueprints/Material/M_Red2_Inst.M_Red2_Inst" 3e+03 false 4.0 2e+01 0)
        (goto _label)))))

(event Custom|Animate
  (bind _scene (Variables|Default|GetScene))
  (bind _returnvalue (Transformation|GetWorldLocation _scene))
  ;[1 1 1] Animate
  (Rendering|SetVisibility (Variables|Default|GetSphere) true false)
  (Utilities|FlowControl|DoOnce false
    (:Completed
      (bind (_direction _z _scale) (Timeline|Timeline_0 PlayFromStart)
        (:Update
          (Transformation|SetWorldTransform _scene (Math|Transform|MakeTransform (Math|Vector|MakeVector (.x _returnvalue) (.y _returnvalue) (+ _z (Variables|Default|GetDistance))) (Transformation|GetWorldRotation _scene) (* "1.000000,1.000000,1.000000" _scale)) false false))
        (:Finished
          ;[1 1 1] Shoot
          (bind _output_get (Variables|Default|SetLookOnCharacter true))
          (if _output_get :!label _label
            (Utilities|FlowControl|Delay 0.5)
            (Game|SpawnActorfromClass "/Game/Blueprints/BP_Bullet.BP_Bullet_C" (Transformation|GetWorldTransform (Variables|Default|GetScene1)) "Undefined" 0 "/Game/Blueprints/Material/M_Red2_Inst.M_Red2_Inst" 3e+03 false 4.0 2e+01 0)
            (goto _label)))))))

(event Custom|StopShoot
  (bind _scene (Variables|Default|GetScene))
  ;[1 1 1] StopShoot
  (Variables|Default|SetLookOnCharacter false)
  (bind _scale (Timeline|Timeline_2 ReverseFromEnd)
    (:Update
      (Transformation|SetWorldTransform _scene (Math|Transform|MakeTransform (Transformation|GetWorldLocation _scene) (Transformation|GetWorldRotation _scene) (* "1.000000,1.000000,1.000000" _scale)) false false))))

(event EventTick
  (params (DeltaSeconds :type Float%20%28single-precision%29))
  ;[1 1 1] Look on Character
  (bind _asfpscharacter (Utilities|Casting|CastToFPSCharacter (Game|Player|GetPlayerPawn 0)))
  (bind _output_get (Variables|Default|SetFPSCharacterWorldLocation (Transformation|GetWorldLocation (Variables|/Script/Engine.Actor|GetRootComponent _asfpscharacter))))
  (Transformation|SetRelativeRotation (Variables|Default|GetSphere) (Math|Rotator|FindLookatRotation (Transformation|GetWorldLocation (Variables|Default|GetSphere)) _output_get) false false))

(fn ConstructionScript)