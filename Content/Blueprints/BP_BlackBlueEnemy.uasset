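; Enemy emplacement actor that wraps a BP_Enemy child actor and drives its entrance, shooting and exit.
; On BeginPlay it binds to a Collision reference's start/stop shooting dispatchers, destroying itself if that is invalid outside DebugMode.
; The first start event reveals the meshes, moves the scene in Z via a reversed timeline, then animates the enemy; later ones shoot.
; Tick detects the enemy's loss, plays an exit timeline and destroys the actor.
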(event Custom|StartShoot
  (bind _scene (Variables|Default|GetScene))
  (bind _bp_enemy (Variables|Default|GetBP_Enemy))
  (bind _returnvalue (Transformation|GetWorldLocation _scene))
  (bind _childactor (Variables|/Script/Engine.ChildActorComponent|GetChildActor _bp_enemy))
  (bind _asbp_enemy (Utilities|Casting|CastToBP_Enemy _childactor))
  ;[1 1 1] Start shoot
  (if (Variables|Default|GetIsAnimate)
    (Default|Shoot _asbp_enemy)
    (else
      (Utilities|FlowControl|DoOnce false
        (:Completed
          (Rendering|SetVisibility (Variables|Default|GetCube1) true false)
          (bind _z (Timeline|Timeline_0 ReverseFromEnd)
            (:Update
              (Transformation|SetWorldTransform _scene (Math|Transform|MakeTransform (Math|Vector|MakeVector (.x _returnvalue) (.y _returnvalue) (+ _z (Variables|Default|GetDistance))) (Transformation|GetWorldRotation _scene) "1,1,1") false false))
            (:Finished
              (Variables|Default|SetIsAnimate true)
              (Default|Animate _asbp_enemy))))))))

(event Custom|CustomEvent_0
  ;[1 1 1] Stop shoot
  (Default|StopShoot (.AsBP%20Enemy (Utilities|Casting|CastToBP_Enemy (Variables|/Script/Engine.ChildActorComponent|GetChildActor (Variables|Default|GetBP_Enemy))))))

(event EventBeginPlay
  (bind _collision (Variables|Default|GetCollision))
  ;[1 1 1] Bind dispatchers
  (Variables|/Game/Blueprints/BP_Enemy.BP_Enemy_C|SetDistance (.AsBP%20Enemy (Utilities|Casting|CastToBP_Enemy (Variables|/Script/Engine.ChildActorComponent|GetChildActor (Variables|Default|GetBP_Enemy)))) (Variables|Default|GetDistance))
  (if (not (Variables|Default|GetDebugMode))
    (Utilities|IsValid _collision
      (:Is%20Valid
        (EventDispatchers|BindEventtoStartShoot _collision (delegate Custom|StartShoot))
        (EventDispatchers|BindEventtoStopShooting _collision (delegate Custom|CustomEvent_0)))
      (:Is%20Not%20Valid
        (Actor|DestroyActor)))))

(event EventTick
  (params (DeltaSeconds :type Float%20%28single-precision%29))
  (bind _scene (Variables|Default|GetScene))
  (bind _returnvalue (Transformation|GetWorldLocation _scene))
  ;[1 1 1] Is Enemy isnt valid
  (Utilities|IsValid (Variables|/Script/Engine.ChildActorComponent|GetChildActor (Variables|Default|GetBP_Enemy))
    (:Is%20Not%20Valid
      (Utilities|FlowControl|DoOnce false
        (:Completed
          (bind _z (Timeline|Timeline_1 PlayFromStart)
            (:Update
              (Transformation|SetWorldTransform _scene (Math|Transform|MakeTransform (Math|Vector|MakeVector (.x _returnvalue) (.y _returnvalue) (+ _z (Variables|Default|GetDistance))) (Transformation|GetWorldRotation _scene) "1,1,1") false false))
            (:Finished
              (Actor|DestroyActor))))))))

(fn ConstructionScript)